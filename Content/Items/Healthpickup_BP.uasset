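; Health pickup actor that restores a player's health when walked over.
; On sphere overlap it casts to Player_BP and, unless health is already full, adds Healthtogive clamped to the player's max.
; It then tells the player's HUD to show a heart with that amount and destroys itself, so full-health players leave it in the world.
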(event `self.Sphere.OnComponentBeginOverlap`
  (params (OverlappedComponent :type "PrimitiveComponent Object Reference") (OtherActor :type "Actor Object Reference") (OtherComp :type "PrimitiveComponent Object Reference") (OtherBodyIndex :type Integer) (bFromSweep :type Boolean) (SweepResult :type "HitResult Structure (by ref)"))
  (bind _as_player_bp (`self.As Player BP`))
  (bind _asplayer_bp (cast `/Game/PlayerCharacter/Player_BP` OtherActor))
  (bind _output_get (set `self.As Player BP` _asplayer_bp))
  (if (not (== (`/Game/PlayerCharacter/Player_BP.health` _output_get) (`/Game/PlayerCharacter/Player_BP.Maxhealth` _output_get)))
    (set `/Game/PlayerCharacter/Player_BP.health` (`KismetMathLibrary.FClamp` (+ (`/Game/PlayerCharacter/Player_BP.health` _as_player_bp) (`self.healthtogive`)) 1.0 (`/Game/PlayerCharacter/Player_BP.Maxhealth` _as_player_bp)) _as_player_bp)
    (`/Game/Widgetblueprints/PlayerHud_WB.Showheart` (`/Game/PlayerCharacter/Player_BP.hudref` (`self.As Player BP`)) (`KismetMathLibrary.FTrunc` (`self.healthtogive`)))
    (`self.K2_DestroyActor`)))

(fn `UserConstructionScript`)