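; Side-scrolling boss character that chases the player along X, flips to face them and attacks with projectiles.
; A randomly seeded looping timer jumps the animation state machine to attack, while a separate Attack event spawns the player-aimed projectile.
; Damage updates the HUD health bar, knocks the boss back, then restores Flying mode.
; Death plays an animation, saves a level flag and opens the main menu.
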(event `handleroation`
  (bind _returnvalue_x (`KismetMathLibrary.BreakVector` (`KismetMathLibrary.GetDirectionUnitVector` (`self.K2_GetActorLocation` (`GameplayStatics.GetPlayerCharacter` 0)) (`self.K2_GetActorLocation`))))
  ;[1 1 1] Hnadle rotation
  (if (`self.isdead`)
    _
    (elif (< _returnvalue_x 0.0)
      (`self.K2_SetActorRotation` (struct))
      (else
        (`self.K2_SetActorRotation` (struct :`Yaw` 180.0))))))

(event `self.ReceiveTick`
  (params (DeltaSeconds :type "Float (single-precision)"))
  (bind (_returnvalue_x _returnvalue_y _returnvalue_z) (`KismetMathLibrary.BreakVector` (- (`self.K2_GetActorLocation` (`GameplayStatics.GetPlayerCharacter` 0)) (`self.K2_GetActorLocation`))))
  (bind _returnvalue_x_2 (`KismetMathLibrary.BreakVector` (`KismetMathLibrary.Normal` (`KismetMathLibrary.MakeVector` _returnvalue_x _returnvalue_y _returnvalue_z))))
  ;[1 1 1] Handle Movement
  (if (not (`self.isdead`))
    (`self.handleroation`)
    (if (not (< (`KismetMathLibrary.Abs` _returnvalue_x) 450.0))
      (`self.AddMovementInput` (1.0 0.0 0.0) _returnvalue_x_2))))

(event `self.ReceiveBeginPlay`
  ;[1 1 1] Show Boss Hud
  (set `self.Maxhealth` (`self.health`))
  (bind _returnvalue (`|CreateWidget` "/Game/Widgetblueprints/BossHealthbar_WB.Bosshealthbar_WB_C" null self))
  (bind _output_get (set `self.bosshudref` _returnvalue))
  (`UserWidget.AddToViewport` _output_get 0)
  ;[1 1 1] Handle Boss Attack
  (bind _returnvalue_2 (`KismetSystemLibrary.K2_SetTimerDelegate` (delegate `playbossattackanimation`) (`KismetMathLibrary.RandomFloatInRange` 2.0 4.0) true))
  (set `self.bossattackevent` _returnvalue_2))

(event `playbossattackanimation`
  ;[1 1 1] Handle Boss Attack
  (if (not (or (`self.enemydamaged`) (`self.isdead`)))
    (`PaperZDAnimInstance.JumpToNode` (`PaperZDAnimationComponent.AnimInstance` (`self.AnimationComponent`)) "attack" "None")))

(event `Attack`
  ;[1 1 1] Handle Boss Attack
  ;;[1 1 1] Spawn boss projectile
  (`SceneComponent.K2_SetWorldRotation` (`self.projectilespawnlocation`) (`KismetMathLibrary.FindLookAtRotation` (`self.K2_GetActorLocation`) (`self.K2_GetActorLocation` (`GameplayStatics.GetPlayerCharacter` 0))) false false)
  (`|SpawnActorFromClass` "/Game/Boss/blueprints/bossprojectile_BP.bossprojectile_BP_C" (`SceneComponent.K2_GetComponentToWorld` (`self.projectilespawnlocation`)) "Undefined" "OverrideRootScale" null null))

(event `self.ReceiveAnyDamage`
  (params (Damage :type "Float (single-precision)") (DamageType :type "DamageType Object Reference") (InstigatedBy :type "Controller Object Reference") (DamageCauser :type "Actor Object Reference"))
  (bind _returnvalue_x (`KismetMathLibrary.BreakVector` (`KismetMathLibrary.GetDirectionUnitVector` (`self.K2_GetActorLocation` DamageCauser) (`self.K2_GetActorLocation`))))
  ;[1 1 1] Handle boss damage
  (set `self.health` (- (`self.health`) Damage))
  (set `self.enemydamaged` true)
  (`/Game/Widgetblueprints/BossHealthbar_WB.Updatehealthbar` (`self.bosshudref`))
  (`self.LaunchCharacter` (`KismetMathLibrary.MakeVector` (* (select `bool` (< _returnvalue_x 0.0) :`false` -1.0 :`true` 1.0) -1200.0) 0.0 300.0) true true)
  (`|ExecutionSequence`
    (:`then_0`
      (if (<= (`self.health`) 0.0)
        (set `self.isdead` true)
        (`Widget.RemoveFromParent` (`self.bosshudref`))
        (`PaperZDAnimInstance.JumpToNode` (`PaperZDAnimationComponent.AnimInstance` (`self.AnimationComponent`)) "die" "None")
        (`KismetSystemLibrary.Delay` 2.0)
        (bind _asplayer_bp (cast `/Game/PlayerCharacter/Player_BP` (`GameplayStatics.GetPlayerCharacter` 0)))
        (bind _as_playersave (`/Game/PlayerCharacter/Player_BP.As Playersave` _asplayer_bp))
        (`KismetArrayLibrary.Array_Set` (`/Game/PlayerCharacter/Playersave.levels` _as_playersave) 2 true)
        (`GameplayStatics.SaveGameToSlot` _as_playersave "1")
        (`GameplayStatics.OpenLevel` "mainmenumap")
        (else
          (`PaperZDAnimInstance.JumpToNode` (`PaperZDAnimationComponent.AnimInstance` (`self.AnimationComponent`)) "damaged" "None")
          (`KismetSystemLibrary.RetriggerableDelay` 1.0)
          (set `self.enemydamaged` false))))
    (:`then_1`
      (`KismetSystemLibrary.Delay` 0.7)
      (`CharacterMovementComponent.SetMovementMode` (`self.CharacterMovement`) "MOVE_Flying" 0))))

(fn `NewFunction_0`)

(fn `UserConstructionScript`)