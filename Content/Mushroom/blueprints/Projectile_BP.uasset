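; Mushroom enemy projectile actor that damages the player on contact and explodes when it hits the player or level geometry.
; Sphere overlap applies a single point of damage to the player, guarded by a DoOnce, or reacts to actors tagged "level" without dealing damage.
; Both paths swap the Paper2D flipbook to the explosion animation, wait for its length, then destroy the actor.
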(event `self.Sphere.OnComponentBeginOverlap`
  (params (OverlappedComponent :type "PrimitiveComponent Object Reference") (OtherActor :type "Actor Object Reference") (OtherComp :type "PrimitiveComponent Object Reference") (OtherBodyIndex :type Integer) (bFromSweep :type Boolean) (SweepResult :type "HitResult Structure (by ref)"))
  (bind _returnvalue (`GameplayStatics.GetPlayerCharacter` 0))
  (if (== OtherActor _returnvalue)
    (`/Engine/EditorBlueprintResources/StandardMacros.DoOnce` false
      (:`Completed`
        (`GameplayStatics.ApplyDamage` _returnvalue 1.0)
        (`PaperFlipbookComponent.SetFlipbook` (`self.PaperFlipbook`) "/Game/Mushroom/Flipbooks/RangedAttack/Mushroomprojectileexplode.Mushroomprojectileexplode" :!label _label)
        (`KismetSystemLibrary.Delay` (`PaperFlipbookComponent.GetFlipbookLength` (`self.PaperFlipbook`)))
        (`self.K2_DestroyActor`)))
    (elif (`self.ActorHasTag` OtherActor "level")
      (goto _label))))

(fn `UserConstructionScript`)